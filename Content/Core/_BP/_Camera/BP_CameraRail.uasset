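; BP_CameraRail is a rail camera that takes over the view when the player character enters its trigger box.
; The overlap stores the player as target, starts a fast looping timer and switches the player controller's view target to this actor.
; Each tick of the timer maps the player's clamped distance from the actor onto the spline's length, moves the camera there and turns it toward the player.
; Leaving the box does nothing.
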(event `ActivateCamera`
  (`KismetSystemLibrary.K2_SetTimerDelegate` (delegate `UpdateCameraLocationAlongSpine`) 0.01 true))

(event `UpdateCameraLocationAlongSpine`
  (bind _railsplinecomponent (`self.RailSplineComponent`))
  (bind _camera (`self.Camera`))
  (`SceneComponent.K2_SetWorldLocation` (`self.Camera`) (`SplineComponent.GetLocationAtDistanceAlongSpline` _railsplinecomponent (* (`SplineComponent.GetSplineLength` _railsplinecomponent) (`KismetMathLibrary.FClamp` (/ (`self.GetDistanceTo` (`self.TargetActor`) self) 2000.0))) "World") false false)
  (`SceneComponent.K2_SetWorldRotation` _camera (`KismetMathLibrary.FindLookAtRotation` (`SceneComponent.K2_GetComponentLocation` _camera) (`SceneComponent.K2_GetComponentLocation` (`Actor.RootComponent` (`self.TargetActor`)))) false false))

(event `self.Box.OnComponentBeginOverlap`
  (params (OverlappedComponent :type "PrimitiveComponent Object Reference") (OtherActor :type "Actor Object Reference") (OtherComp :type "PrimitiveComponent Object Reference") (OtherBodyIndex :type Integer) (bFromSweep :type Boolean) (SweepResult :type "HitResult Structure (by ref)"))
  (bind _asbp_player_character (cast `/Game/Core/_BP/_Player_Character/BP_PlayerCharacter` OtherActor))
  (set `self.TargetActor` _asbp_player_character)
  (`self.ActivateCamera`)
  (`PlayerController.SetViewTargetWithBlend` (`GameplayStatics.GetPlayerController` 0) self 0.0 "VTBlend_Linear" 0.0 false))

(event `self.Box.OnComponentEndOverlap`
  (params (OverlappedComponent :type "PrimitiveComponent Object Reference") (OtherActor :type "Actor Object Reference") (OtherComp :type "PrimitiveComponent Object Reference") (OtherBodyIndex :type Integer)))

(fn `UserConstructionScript`)