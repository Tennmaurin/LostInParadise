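; Trigger volume that changes the player character's camera position values while the player is inside it.
; On begin overlap of its collision component, it copies its own camera height, X and Y variables onto the overlapping BP_PlayerCharacter.
; On end overlap, it writes hardcoded default values back rather than restoring whatever the character had before entering.
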(event `self.CollisionComponent.OnComponentBeginOverlap`
  (params (OverlappedComponent :type "PrimitiveComponent Object Reference") (OtherActor :type "Actor Object Reference") (OtherComp :type "PrimitiveComponent Object Reference") (OtherBodyIndex :type Integer) (bFromSweep :type Boolean) (SweepResult :type "HitResult Structure (by ref)"))
  (bind _asbp_player_character (cast `/Game/Core/_BP/_Player_Character/BP_PlayerCharacter` OtherActor))
  (set `/Game/Core/_BP/_Player_Character/BP_PlayerCharacter.CameraHight` (`self.CameraHight`) _asbp_player_character)
  (set `/Game/Core/_BP/_Player_Character/BP_PlayerCharacter.CameraX` (`self.CameraX`) _asbp_player_character)
  (set `/Game/Core/_BP/_Player_Character/BP_PlayerCharacter.CameraY` (`self.CameraY`) _asbp_player_character))

(event `self.CollisionComponent.OnComponentEndOverlap`
  (params (OverlappedComponent :type "PrimitiveComponent Object Reference") (OtherActor :type "Actor Object Reference") (OtherComp :type "PrimitiveComponent Object Reference") (OtherBodyIndex :type Integer))
  (bind _asbp_player_character (cast `/Game/Core/_BP/_Player_Character/BP_PlayerCharacter` OtherActor))
  (set `/Game/Core/_BP/_Player_Character/BP_PlayerCharacter.CameraHight` 700.0 _asbp_player_character)
  (set `/Game/Core/_BP/_Player_Character/BP_PlayerCharacter.CameraX` -450.0 _asbp_player_character)
  (set `/Game/Core/_BP/_Player_Character/BP_PlayerCharacter.CameraY` 200.0 _asbp_player_character))

(fn `UserConstructionScript`)