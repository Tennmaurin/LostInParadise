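; BP_CameraOnRail is a camera actor that takes over the player's view when BP_PlayerCharacter enters its box, apparently intended to travel along a rail.
; On overlap it stores the character as target, blends the view to itself and starts a fast looping timer.
; The timer only prints the normalized distance to the target and resets the rail position to zero, so rail movement is unfinished.
; Look-at rotation toward the target exists but is disconnected.
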(event `ActivateCamera`
  (`KismetSystemLibrary.K2_SetTimerDelegate` (delegate `UpdateCameraLocationAlongSpine`) 0.01 true))

(event `UpdateCameraLocationAlongSpine`
  (`KismetSystemLibrary.PrintString` (`KismetStringLibrary.Conv_DoubleToString` (`KismetMathLibrary.NormalizeToRange` (`self.GetDistanceTo` (`self.TargetActor`) self) 0.0 1.0)))
  (set `self.CurrentPositionOnRail` 0.0))

(event `self.Box.OnComponentBeginOverlap`
  (params (OverlappedComponent :type "PrimitiveComponent Object Reference") (OtherActor :type "Actor Object Reference") (OtherComp :type "PrimitiveComponent Object Reference") (OtherBodyIndex :type Integer) (bFromSweep :type Boolean) (SweepResult :type "HitResult Structure (by ref)"))
  (bind _asbp_player_character (cast `/Game/Core/_BP/_Player_Character/BP_PlayerCharacter` OtherActor))
  (set `self.TargetActor` _asbp_player_character)
  (`self.ActivateCamera`)
  (`PlayerController.SetViewTargetWithBlend` (`GameplayStatics.GetPlayerController` 0) self 0.0 "VTBlend_Linear" 0.0 false))

(fn `UserConstructionScript`)