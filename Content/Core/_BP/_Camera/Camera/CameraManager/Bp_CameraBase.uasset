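; Base camera actor that becomes the player's view target and follows the player character.
; On BeginPlay it sets itself as the view target and registers as the BP_PlayerCharacter's camera reference.
; Each tick it places the spring arm at the character's capsule location plus world-space X, Y and height offsets read from that character, then rotates it to look at the capsule.
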(event `self.ReceiveBeginPlay`
  (`PlayerController.SetViewTargetWithBlend` (`GameplayStatics.GetPlayerController` 0) self 0.0 "VTBlend_Linear" 0.0 false)
  (bind _asbp_player_character (cast `/Game/Core/_BP/_Player_Character/BP_PlayerCharacter` (`GameplayStatics.GetPlayerCharacter` 0)))
  (set `/Game/Core/_BP/_Player_Character/BP_PlayerCharacter.CameraReference` self _asbp_player_character))

(event `self.ReceiveTick`
  (params (DeltaSeconds :type "Float (single-precision)"))
  (bind _returnvalue (`GameplayStatics.GetPlayerCharacter` 0))
  (bind _springarm (`self.SpringArm`))
  (bind _asbp_player_character (cast `/Game/Core/_BP/_Player_Character/BP_PlayerCharacter` _returnvalue :!pure true))
  (bind _capsulecomponent (`Character.CapsuleComponent` _returnvalue))
  (bind (_returnvalue_x _returnvalue_y _returnvalue_z) (`KismetMathLibrary.BreakVector` (`SceneComponent.K2_GetComponentLocation` _capsulecomponent)))
  (`/Engine/EditorBlueprintResources/StandardMacros.IsValid` _returnvalue
    (:`Is Valid`
      (`SceneComponent.K2_SetWorldLocation` (`self.SpringArm`) (`KismetMathLibrary.MakeVector` (+ _returnvalue_x (`/Game/Core/_BP/_Player_Character/BP_PlayerCharacter.CameraX` _asbp_player_character)) (+ _returnvalue_y (`/Game/Core/_BP/_Player_Character/BP_PlayerCharacter.CameraY` _asbp_player_character)) (+ _returnvalue_z (`/Game/Core/_BP/_Player_Character/BP_PlayerCharacter.CameraHight` _asbp_player_character))) false false)
      (`SceneComponent.K2_SetWorldRotation` _springarm (`KismetMathLibrary.FindLookAtRotation` (`SceneComponent.K2_GetComponentLocation` _springarm) (`SceneComponent.K2_GetComponentLocation` _capsulecomponent)) false false))))

(fn `UserConstructionScript`)