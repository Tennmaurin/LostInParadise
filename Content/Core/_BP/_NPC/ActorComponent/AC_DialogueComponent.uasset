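; NPC actor component that opens a dialogue screen when OnUse fires.
; OnUse creates a dialogue widget for the first player controller, adds it to the viewport and switches input to UI only, focused on the widget without mouse lock.
; The widget's OnExit event is bound back to the component, which restores game-only input for the owning player and removes the widget.
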(event `/Game/Core/_BP/_Interactable_object/Interface_UseObject.OnUse`
  (bind _returnvalue (`GameplayStatics.GetPlayerController` 0))
  (bind _returnvalue_2 (`|GenericCreateObject` "/Game/Core/_BP/_NPC/Widget/_WDG_DialogueWidget._WDG_DialogueWidget_C" _returnvalue))
  (bind _output_get (set `self.DialogueWidget` _returnvalue_2))
  (add `/Game/Core/_BP/_NPC/Widget/_WDG_DialogueWidget.OnExit` _output_get (delegate `OnExit_Event_1`))
  (`UserWidget.AddToViewport` _output_get 0)
  (`WidgetBlueprintLibrary.SetInputMode_UIOnlyEx` _returnvalue _output_get))

(event `OnExit_Event_1`
  (`WidgetBlueprintLibrary.SetInputMode_GameOnly` (`Widget.GetOwningPlayer` (`self.DialogueWidget`)))
  (`Widget.RemoveFromParent` (`self.DialogueWidget`)))