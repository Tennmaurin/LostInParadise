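; Inventory component that holds stackable items in a fixed number of slots and creates the tools HUD widget on BeginPlay.
; Adding flags axe or pickaxe on that widget, then tops up partial stacks, recursing on overflow, or fills an empty slot, reporting success even when full.
; Removal checks totals, then drains matching stacks from the array's end by temporarily reversing it.
; Both fire OnInventoryUpdated; ToggleInventory's window logic is disconnected.
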(event `self.ReceiveBeginPlay`
  (`self.PrepareInventory`)
  (bind _returnvalue (`|CreateWidget` "/Game/Core/_BP/_NewInventorySystem/InventoryUI/WDG_ToolsInventory.WDG_ToolsInventory_C"))
  (bind _output_get (set `self.ToolsWindow` _returnvalue))
  (`UserWidget.AddToViewport` _output_get 0))

(fn `AddToInventory`
  (params (ContentToAdd :type "/Game/Core/_BP/_NewInventorySystem/SlotStructure Structure"))
  (returns (Success :type Boolean))
  (bind _toolswindow (`self.ToolsWindow`))
  (bind _contenttoadd (`local.ContentToAdd`))
  (bind _toolswindow_2 (`self.ToolsWindow`))
  (if (== (`.Class_20_E8CB4C124B4A370253AE42BBE98D0598` (break `/Game/Core/_BP/_NewInventorySystem/ItemStructure` (break `/Game/Core/_BP/_NewInventorySystem/SlotStructure` ContentToAdd))) "/Game/Core/_BP/_NewInventorySystem/Item/BP_Item_Axe.BP_Item_Axe_C")
    (set `/Game/Core/_BP/_NewInventorySystem/InventoryUI/WDG_ToolsInventory.HasAxe` true _toolswindow_2)
    (set `/Game/Core/_BP/_NewInventorySystem/InventoryUI/WDG_ToolsInventory.Min` 0 _toolswindow_2)
    (elif (== (`.Class_20_E8CB4C124B4A370253AE42BBE98D0598` (break `/Game/Core/_BP/_NewInventorySystem/ItemStructure` (break `/Game/Core/_BP/_NewInventorySystem/SlotStructure` ContentToAdd))) "/Game/Core/_BP/_NewInventorySystem/Item/BP_Item_PickAxe.BP_Item_PickAxe_C")
      (set `/Game/Core/_BP/_NewInventorySystem/InventoryUI/WDG_ToolsInventory.HasPickaxe` true _toolswindow)
      (set `/Game/Core/_BP/_NewInventorySystem/InventoryUI/WDG_ToolsInventory.Max` 2 _toolswindow)))
  (if (`.IsStackable_5_074020A943ED1B14D31BF294F993A669` (break `/Game/Core/_BP/_NewInventorySystem/ItemStructure` (break `/Game/Core/_BP/_NewInventorySystem/SlotStructure` ContentToAdd)))
    (bind _stackindex (`self.HasPartialStack` _contenttoadd)
      (:`True`
        (`self.AddToStack` _contenttoadd _stackindex))
      (:`False`
        (`self.CreateStack` _contenttoadd :!label _label)))
    (else
      (goto _label)))
  (`self.OnInventoryUpdated`)
  (return true))

(fn `AddToStack`
  (params (SlotStructure :type "/Game/Core/_BP/_NewInventorySystem/SlotStructure Structure") (SlotIndex :type Integer))
  (returns (Success :type Boolean))
  (locals (CurrentQuantity :type Integer))
  (bind _inventory (`self.Inventory`))
  (bind (_slotstructure_itemstructure _slotstructure_quantity) (break `/Game/Core/_BP/_NewInventorySystem/SlotStructure` (`local.SlotStructure`)))
  (bind _slotindex (`local.SlotIndex`))
  (bind (_slotstructure_itemstructure_2 _slotstructure_quantity_2) (break `/Game/Core/_BP/_NewInventorySystem/SlotStructure` (`local.SlotStructure`)))
  (bind _slotstructure_itemstructure_3 (break `/Game/Core/_BP/_NewInventorySystem/SlotStructure` (`local.SlotStructure`)))
  (bind (_name _isstackable _thumbnail _description _isconsumable _maxstacksize) (break `/Game/Core/_BP/_NewInventorySystem/ItemStructure` _slotstructure_itemstructure_3))
  (bind _output (`|GetArrayItem` (`self.Inventory`) SlotIndex))
  (bind (_output_itemstructure _output_quantity) (break `/Game/Core/_BP/_NewInventorySystem/SlotStructure` (`|GetArrayItem` _inventory _slotindex)))
  (bind _output_get (set `local.CurrentQuantity` (`.Quantity_5_108038A8418761865652A9BFA5CD0F4B` (break `/Game/Core/_BP/_NewInventorySystem/SlotStructure` _output))))
  (if (> (+ _output_get (`.Quantity_5_108038A8418761865652A9BFA5CD0F4B` (break `/Game/Core/_BP/_NewInventorySystem/SlotStructure` SlotStructure))) (`.MaxStackSize_21_F4DAB2BB43EB4F1520ADD7ABD39F684D` (break `/Game/Core/_BP/_NewInventorySystem/ItemStructure` (break `/Game/Core/_BP/_NewInventorySystem/SlotStructure` _output))))
    (`KismetArrayLibrary.Array_Set` (`self.Inventory`) (`local.SlotIndex`) (make `/Game/Core/_BP/_NewInventorySystem/SlotStructure` _slotstructure_itemstructure_3 _maxstacksize))
    (bind _success (`self.AddToInventory` (make `/Game/Core/_BP/_NewInventorySystem/SlotStructure` _slotstructure_itemstructure (- _slotstructure_quantity (- _maxstacksize (`local.CurrentQuantity`))))))
    (else
      (`KismetArrayLibrary.Array_Set` _inventory _slotindex (make `/Game/Core/_BP/_NewInventorySystem/SlotStructure` _output_itemstructure (+ _output_quantity _slotstructure_quantity_2)))))
  (return _success))

(fn `CheckForItem`
  (params (Content :type "/Game/Core/_BP/_NewInventorySystem/Item/BP_Item Class Reference"))
  (returns (Success :type Boolean) (ItemQuantity :type Integer))
  (for _array_element (`self.Inventory`)
    (bind _returnvalue (== (`local.Content`) (`.Class_20_E8CB4C124B4A370253AE42BBE98D0598` (break `/Game/Core/_BP/_NewInventorySystem/ItemStructure` (break `/Game/Core/_BP/_NewInventorySystem/SlotStructure` _array_element)))))
    (if _returnvalue
      (break)))
  (return _returnvalue (`.Quantity_5_108038A8418761865652A9BFA5CD0F4B` (break `/Game/Core/_BP/_NewInventorySystem/SlotStructure` _array_element))))

(fn `CreateStack`
  (params (ContentToAdd :type "/Game/Core/_BP/_NewInventorySystem/SlotStructure Structure"))
  (returns (Success :type Boolean))
  (locals (HasSpace :type Boolean) (IdentifiedIndex :type Integer))
  (for (_array_element _array_index) (`self.Inventory`)
    (if (<= (`.Quantity_5_108038A8418761865652A9BFA5CD0F4B` (break `/Game/Core/_BP/_NewInventorySystem/SlotStructure` _array_element)) 0)
      (set `local.HasSpace` true)
      (set `local.IdentifiedIndex` _array_index)
      (break)))
  (if (`local.HasSpace`)
    (`KismetArrayLibrary.Array_Set` (`self.Inventory`) (`local.IdentifiedIndex`) (`local.ContentToAdd`))
    (return (`local.HasSpace`))
    (else
      (return false))))

(fn `Delete Stack`
  (params (StackIndex :type Integer))
  (`KismetArrayLibrary.Array_Set` (`self.Inventory`) StackIndex (make `/Game/Core/_BP/_NewInventorySystem/SlotStructure` (struct :`Name` "NSLOCTEXT(\"[669252404588E9891740FE809109BB2F]\", \"EACF22D54303E58203EB1CB20717650E\", \"None\")" :`IsStackable` true :`Description` "NSLOCTEXT(\"[669252404588E9891740FE809109BB2F]\", \"555DBD9443ED757112C51B8C80FDF2DA\", \"None\")" :`IsConsumable` true :`MaxStackSize` 64))))

(fn `PrepareInventory`
  (`KismetArrayLibrary.Array_Resize` (`self.Inventory`) (`self.NumberOfSlots`)))

(fn `RemoveFromInventory`
  (params (ContentToRemove :type "/Game/Core/_BP/_NewInventorySystem/SlotStructure Structure"))
  (returns (Success :type Boolean))
  (bind _success (`self.HasEnough` ContentToRemove)
    (:`Out`
      (if _success
        (`self.RemoveFromStack` (`local.ContentToRemove`))
        (return true)
        (else
          (return false))))))

(fn `RemoveFromStack`
  (params (ContentToRemove :type "/Game/Core/_BP/_NewInventorySystem/SlotStructure Structure"))
  (locals (Quantity :type Integer))
  (bind _inventory (`self.Inventory`))
  (bind (_contenttoremove_itemstructure _contenttoremove_quantity) (break `/Game/Core/_BP/_NewInventorySystem/SlotStructure` (`local.ContentToRemove`)))
  (set `local.Quantity` ContentToRemove_Quantity_5_108038A8418761865652A9BFA5CD0F4B)
  (`KismetArrayLibrary.Array_Reverse` _inventory)
  (for (_array_element _array_index) _inventory
    (if (== (`.Class_20_E8CB4C124B4A370253AE42BBE98D0598` (break `/Game/Core/_BP/_NewInventorySystem/ItemStructure` (break `/Game/Core/_BP/_NewInventorySystem/SlotStructure` (`local.ContentToRemove`)))) (`.Class_20_E8CB4C124B4A370253AE42BBE98D0598` (break `/Game/Core/_BP/_NewInventorySystem/ItemStructure` (break `/Game/Core/_BP/_NewInventorySystem/SlotStructure` _array_element))))
      (if (>= (`local.Quantity`) (`.Quantity_5_108038A8418761865652A9BFA5CD0F4B` (break `/Game/Core/_BP/_NewInventorySystem/SlotStructure` _array_element)))
        (bind _output_get (set `local.Quantity` (- (`local.Quantity`) (`.Quantity_5_108038A8418761865652A9BFA5CD0F4B` (break `/Game/Core/_BP/_NewInventorySystem/SlotStructure` _array_element)))))
        (`self.Delete Stack` _array_index)
        (if (not (> _output_get 0))
          (break))
        (else
          (`KismetArrayLibrary.Array_Set` (`self.Inventory`) _array_index (make `/Game/Core/_BP/_NewInventorySystem/SlotStructure` _contenttoremove_itemstructure (- (`.Quantity_5_108038A8418761865652A9BFA5CD0F4B` (break `/Game/Core/_BP/_NewInventorySystem/SlotStructure` _array_element)) _contenttoremove_quantity)))
          (break)))))
  (`KismetArrayLibrary.Array_Reverse` (`self.Inventory`))
  (`self.OnInventoryUpdated`)
  (return))

(fn `ToggleInventory`)