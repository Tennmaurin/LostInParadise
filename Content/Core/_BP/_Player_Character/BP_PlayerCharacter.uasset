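; BP_PlayerCharacter is the player character, able to move and to take control of an interactable object.
; Axis inputs move it along fixed world X and Y axes, independent of camera or control rotation.
; Pressing E while OnRangeToUseObject is set calls OnUse, which blends the view to ObjectToInteract, waits for the blend duration, then has the player controller possess that object.
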(event `InputAxis|MoveForward`
  (params (AxisValue :type "Float (single-precision)"))
  (`self.AddMovementInput` (90.0 0.0 0.0) AxisValue))

(event `InputAxis|MoveRight`
  (params (AxisValue :type "Float (single-precision)"))
  (`self.AddMovementInput` (0.0 90.0 0.0) AxisValue))

(event `Key|E`
  (params (Key :type "Key Structure"))
  (:`Pressed`
    (if (`self.OnRangeToUseObject?`)
      (`self.OnUse`))))

(event `self.OnUse`
  (bind _returnvalue (`GameplayStatics.GetPlayerController` 0))
  (bind _objecttointeract (`self.ObjectToInteract`))
  (`PlayerController.SetViewTargetWithBlend` _returnvalue _objecttointeract 1.0 "VTBlend_Linear" 0.0 false)
  (`KismetSystemLibrary.Delay` 1.0)
  (`Controller.Possess` _returnvalue _objecttointeract))

(fn `UserConstructionScript`)