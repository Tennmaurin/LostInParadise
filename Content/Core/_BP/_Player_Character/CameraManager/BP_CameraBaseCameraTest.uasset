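; Test camera actor that becomes player 0's view target and follows the player character.
; On BeginPlay it also registers itself as CameraReference on BP_PlayerCharacterCameraTest.
; Each tick it places its SpringArm at the capsule's world location plus the character's CameraX, CameraY and CameraHight offsets, then rotates it to look at the capsule.
; Offsets apply along world axes and movement is set directly, without interpolation.
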(event `self.ReceiveBeginPlay`
  (`PlayerController.SetViewTargetWithBlend` (`GameplayStatics.GetPlayerController` 0) self 0.0 "VTBlend_Linear" 0.0 false)
  (bind _asbp_player_character_camera_test (cast `/Game/Core/_BP/_Player_Character/BP_PlayerCharacterCameraTest` (`GameplayStatics.GetPlayerCharacter` 0)))
  (set `/Game/Core/_BP/_Player_Character/BP_PlayerCharacterCameraTest.CameraReference` self _asbp_player_character_camera_test))

(event `self.ReceiveTick`
  (params (DeltaSeconds :type "Float (single-precision)"))
  (bind _returnvalue (`GameplayStatics.GetPlayerCharacter` 0))
  (bind _springarm (`self.SpringArm`))
  (bind _asbp_player_character_camera_test (cast `/Game/Core/_BP/_Player_Character/BP_PlayerCharacterCameraTest` _returnvalue :!pure true))
  (bind _capsulecomponent (`Character.CapsuleComponent` _returnvalue))
  (bind (_returnvalue_x _returnvalue_y _returnvalue_z) (`KismetMathLibrary.BreakVector` (`SceneComponent.K2_GetComponentLocation` _capsulecomponent)))
  (`/Engine/EditorBlueprintResources/StandardMacros.IsValid` _returnvalue
    (:`Is Valid`
      (`SceneComponent.K2_SetWorldLocation` (`self.SpringArm`) (`KismetMathLibrary.MakeVector` (+ _returnvalue_x (`/Game/Core/_BP/_Player_Character/BP_PlayerCharacterCameraTest.CameraX` _asbp_player_character_camera_test)) (+ _returnvalue_y (`/Game/Core/_BP/_Player_Character/BP_PlayerCharacterCameraTest.CameraY` _asbp_player_character_camera_test)) (+ _returnvalue_z (`/Game/Core/_BP/_Player_Character/BP_PlayerCharacterCameraTest.CameraHight` _asbp_player_character_camera_test))) false false)
      (`SceneComponent.K2_SetWorldRotation` _springarm (`KismetMathLibrary.FindLookAtRotation` (`SceneComponent.K2_GetComponentLocation` _springarm) (`SceneComponent.K2_GetComponentLocation` _capsulecomponent)) false false))))

(fn `UserConstructionScript`)