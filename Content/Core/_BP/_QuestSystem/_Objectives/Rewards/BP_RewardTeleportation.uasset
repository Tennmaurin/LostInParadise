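; Quest reward that, when activated, teleports the player and the Father, Mother and Girl NPCs to placed position markers behind a screen transition.
; It destroys and respawns the Father at his marker, then retargets and updates a hard-indexed talk objective in the player's first quest to the new instance.
; After the transition out, Mother and Girl switch to their finishing dialogue trees.
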(event `self.ActivateReward`
  (bind _fatherpos (`self.FatherPos`))
  (bind _playerpos (`self.PlayerPos`))
  (bind _motherpos (`self.MotherPos`))
  (bind _girlpos (`self.GirlPos`))
  (bind _as_bp_player_character (cast `/Game/Core/_BP/_Player_Character/_BP_PlayerCharacter` (`GameplayStatics.GetPlayerPawn` 0) :!pure true))
  (bind _asbp_obj_talk (cast `/Game/Core/_BP/_QuestSystem/_Objectives/BP_ObjTalk` (`|GetArrayItem` (`/Game/Core/_BP/_QuestSystem/_Objectives/_BP_ObjCollection.Objectives` (`/Game/Core/_BP/_QuestSystem/_Quests/_BP_Quest.RootObjectiveCollection` (`|GetArrayItem` (`/Game/Core/_BP/_QuestSystem/_BP_QuestComponent.Quests` (`/Game/Core/_BP/_Player_Character/_BP_PlayerCharacter._BP_QuestComponent` _as_bp_player_character))))) 10) :!pure true))
  (`KismetSystemLibrary.Delay` 1.0)
  (`/Game/Core/_BP/_Player_Character/_BP_PlayerCharacter.TransiIn` (cast `/Game/Core/_BP/_Player_Character/_BP_PlayerCharacter` (`GameplayStatics.GetPlayerPawn` 0) :!pure true))
  (`KismetSystemLibrary.Delay` 1.5)
  (`self.K2_TeleportTo` (cast `/Game/Core/_BP/_Player_Character/_BP_PlayerCharacter` (`GameplayStatics.GetPlayerPawn` 0) :!pure true) (`self.K2_GetActorLocation` _playerpos) (`self.K2_GetActorRotation` _playerpos))
  (`self.K2_TeleportTo` (`self.Father`) (`self.K2_GetActorLocation` _fatherpos) (`self.K2_GetActorRotation` _fatherpos))
  (`self.K2_TeleportTo` (`self.Mother`) (`self.K2_GetActorLocation` _motherpos) (`self.K2_GetActorRotation` _motherpos))
  (`self.K2_TeleportTo` (`self.Girl`) (`self.K2_GetActorLocation` _girlpos) (`self.K2_GetActorRotation` _girlpos))
  (`self.K2_DestroyActor` (`self.Father`))
  (bind _returnvalue (`|SpawnActorFromClass` "/Game/Core/_BP/NPC/BP/BP_NPC_Father.BP_NPC_Father_C" (`self.GetTransform` (`self.FatherPos`)) "Undefined" "OverrideRootScale" null null))
  (bind _output_get (set `self.Father` _returnvalue))
  (set `/Game/Core/_BP/_QuestSystem/_Objectives/BP_ObjTalk.TalkTarget` _output_get _asbp_obj_talk)
  (`/Game/Core/_BP/_QuestSystem/_Objectives/BP_ObjTalk.UpdateObjective` _asbp_obj_talk)
  (`/Game/Core/_BP/_Player_Character/_BP_PlayerCharacter.TransiOut` _as_bp_player_character)
  (set `/Game/Core/_BP/NPC/BP/BP_NPC.DialogTree` "/Game/Core/_BP/NPC/Dialogue/BT_MotherFinish.BT_MotherFinish" (`self.Mother`))
  (set `/Game/Core/_BP/NPC/BP/BP_NPC.DialogTree` "/Game/Core/_BP/NPC/Dialogue/BT_GirlFinish.BT_GirlFinish" (`self.Girl`)))

(fn `UserConstructionScript`
  (`parent.UserConstructionScript`))