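; BP_NPCManagers swaps the state of the father and mother NPCs when a specific objective in the player's quest completes.
; After a short delay on BeginPlay, it binds to the fifth objective of the first quest on the player character's quest component.
; On completion, it assigns search dialog trees to both parents and gives the father new waypoints, then refreshes his path.
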(event `self.ReceiveBeginPlay`
  (`KismetSystemLibrary.Delay` 2.0)
  (add `/Game/Core/_BP/_QuestSystem/_Objectives/_BP_Objective.OnCompleted` (`|GetArrayItem` (`/Game/Core/_BP/_QuestSystem/_Objectives/_BP_ObjCollection.Objectives` (`/Game/Core/_BP/_QuestSystem/_Quests/_BP_Quest.RootObjectiveCollection` (`|GetArrayItem` (`/Game/Core/_BP/_QuestSystem/_BP_QuestComponent.Quests` (`/Game/Core/_BP/_Player_Character/_BP_PlayerCharacter._BP_QuestComponent` (cast `/Game/Core/_BP/_Player_Character/_BP_PlayerCharacter` (`GameplayStatics.GetPlayerPawn` 0) :!pure true)))))) 4) (delegate `Quest5Complete`))
  (`KismetSystemLibrary.PrintString` "success"))

(event `Quest5Complete`
  (params (Objective :type "/Game/Core/_BP/_QuestSystem/_Objectives/_BP_Objective Object Reference"))
  (`self.Update Quest 5`))

(event `Update Quest 5`
  (bind _npc_father (`self.NPC_Father`))
  (set `/Game/Core/_BP/NPC/BP/BP_NPC.DialogTree` (`self.Dialog_Father_Search`) (`self.NPC_Father`))
  (set `/Game/Core/_BP/NPC/BP/BP_NPC.DialogTree` (`self.Dialog_Mother_Search`) (`self.NPC_Mother`))
  (set `/Game/Core/_BP/NPC/BP/BP_NPC.Waypoints` (`self.Waypoint_Father_Search`) _npc_father)
  (`/Game/Core/_BP/NPC/BP/BP_NPC.UpdateWaypoints` _npc_father))

(fn `UserConstructionScript`)