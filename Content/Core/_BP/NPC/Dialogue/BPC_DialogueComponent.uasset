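; Actor component that runs NPC dialogue by executing a behavior tree on a dedicated AIC_Dialogue controller spawned at BeginPlay.
; StartDialogue opens the dialogue widget, passes widget, NPC and name to the tree's blackboard, blocks player movement and optionally switches to the dialogue camera.
; ExitDialogue stops the tree, removes the widget and restores player movement and camera.
; The widget reference doubles as the guard against starting or exiting twice.
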(event `self.ReceiveBeginPlay`
  (bind _returnvalue (`|SpawnActorFromClass` "/Game/Core/_BP/NPC/ActorComponent/AIC_Dialogue.AIC_Dialogue_C" (`KismetMathLibrary.MakeTransform` (0.0 0.0 0.0)) "Undefined" "OverrideRootScale" null null))
  (set `self.DialogueAIController` _returnvalue))

(event `StartDialogue`
  (params (`Dialogue Tree` :type "BehaviorTree Object Reference") (`IsCameraChanging?` :type Boolean) (`Dialogue Owner` :type "Object Object Reference") (`Target Name` :type String))
  (bind _dialogueaicontroller (`self.DialogueAIController`))
  (bind _as_bp_player_character (cast `/Game/Core/_BP/_Player_Character/_BP_PlayerCharacter` (`GameplayStatics.GetPlayerPawn` 0) :!pure true))
  (`/Engine/EditorBlueprintResources/StandardMacros.IsValid` (`self.DialogWidget`)
    (:`Is Not Valid`
      (bind _returnvalue (`|GenericCreateObject` "/Game/Core/_BP/NPC/Widget/WDG_DialogueWidget.WDG_DialogueWidget_C" (cast `/Game/Core/_BP/_NewInventorySystem/MyPlayerController` (`GameplayStatics.GetPlayerController` 0) :!pure true)))
      (bind _output_get (set `self.DialogWidget` _returnvalue))
      (`UserWidget.AddToViewport` _output_get 0)
      (`/Game/Core/_BP/_Player_Character/_BP_PlayerCharacter.BlockMovements` (cast `/Game/Core/_BP/_Player_Character/_BP_PlayerCharacter` (`GameplayStatics.GetPlayerPawn` 0) :!pure true))
      (`AIController.RunBehaviorTree` _dialogueaicontroller `Dialogue Tree`)
      (bind _blackboardcomponent (`AIController.UseBlackboard` _dialogueaicontroller "/Game/Core/_BP/NPC/Dialogue/BB_DialogueTree.BB_DialogueTree"))
      (`BlackboardComponent.SetValueAsObject` _blackboardcomponent "DialogWidget" (`self.DialogWidget`))
      (`BlackboardComponent.SetValueAsObject` _blackboardcomponent "NPC" `Dialogue Owner`)
      (`BlackboardComponent.SetValueAsString` _blackboardcomponent "NpcName" `Target Name`)
      (`WidgetBlueprintLibrary.SetInputMode_GameAndUIEx` (cast `/Game/Core/_BP/_NewInventorySystem/MyPlayerController` (`GameplayStatics.GetPlayerController` 0) :!pure true) (`self.DialogWidget`))
      (set `/Game/Core/_BP/_Player_Character/_BP_PlayerCharacter.OnDialogueWithNPC` true _as_bp_player_character)
      (if `IsCameraChanging?`
        (`/Game/Core/_BP/_Player_Character/_BP_PlayerCharacter.SetDialogueCamera` _as_bp_player_character)))))

(event `ExitDialogue`
  (bind _as_bp_player_character (cast `/Game/Core/_BP/_Player_Character/_BP_PlayerCharacter` (`GameplayStatics.GetPlayerPawn` 0) :!pure true))
  (`/Engine/EditorBlueprintResources/StandardMacros.IsValid` (`self.DialogWidget`)
    (:`Is Valid`
      (`/Game/Core/_BP/_Player_Character/_BP_PlayerCharacter.RestartMovements` _as_bp_player_character)
      (`BrainComponent.StopLogic` (`AIController.BrainComponent` (`self.DialogueAIController`)) "")
      (`Widget.RemoveFromParent` (`self.DialogWidget`))
      (set `self.DialogWidget` null)
      (set `/Game/Core/_BP/_Player_Character/_BP_PlayerCharacter.OnDialogueWithNPC` false _as_bp_player_character)
      (`/Game/Core/_BP/_Player_Character/_BP_PlayerCharacter.ExitDialogueCam` _as_bp_player_character))))