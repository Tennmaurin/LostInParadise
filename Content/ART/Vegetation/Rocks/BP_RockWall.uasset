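; BP_RockWall is an environment actor that procedurally builds a rock wall along a spline in its construction script.
; It places a static mesh component every DistancePerRock along the spline, each with random roll and pitch bounded by RandomX and RandomY.
; A second pass links consecutive rock positions with manually attached spline mesh components, created at a RockHeight Z offset.
; The random height jitter on those segment endpoints has a zero range, and the event graph is unused.
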(fn `UserConstructionScript`
  (bind _instancemesh (`self.InstanceMesh`))
  (bind _random_x (`self.Random X`))
  (bind _random_y (`self.Random Y`))
  (`|ExecutionSequence`
    (:`then_0`
      (`KismetArrayLibrary.Array_Clear` (`self.InstanceMesh`))
      (for _index (range (`KismetMathLibrary.FFloor` (/ (`SplineComponent.GetSplineLength` (`self.Spline`)) (`self.DistancePerRock`))))
        (bind _returnvalue (`AddComponent|NODE_AddStaticMeshComponent-0`))
        (`SceneComponent.K2_SetWorldLocation` _returnvalue (`SplineComponent.GetLocationAtDistanceAlongSpline` (`self.Spline`) (* _index (`self.DistancePerRock`)) "World") false false)
        (`SceneComponent.K2_AddWorldRotation` _returnvalue (`KismetMathLibrary.MakeRotator` (`KismetMathLibrary.RandomFloatInRange` (* _random_x 0.0) _random_x) (`KismetMathLibrary.RandomFloatInRange` (* _random_y 0.0) _random_y)) false false)
        (`KismetArrayLibrary.Array_Add` (`self.InstanceMesh`) _returnvalue)))
    (:`then_1`
      (`KismetArrayLibrary.Array_Clear` (`self.InstanceSplineMesh`))
      (for (_array_element _array_index) _instancemesh
        (bind _returnvalue_2 (`AddComponent|NODE_AddSplineMeshComponent-0` :`bManualAttachment` true :`RelativeTransform` (`KismetMathLibrary.MakeTransform` (`KismetMathLibrary.MakeVector` 0.0 0.0 (`self.Rock Height`)) (struct) (1.0 1.0 1.0))))
        (bind _returnvalue_3 (+ _array_index 1))
        (if (`KismetArrayLibrary.Array_IsValidIndex` _instancemesh _returnvalue_3)
          (`SplineMeshComponent.SetStartAndEnd` _returnvalue_2 (+ (`SceneComponent.K2_GetComponentLocation` _array_element) (`KismetMathLibrary.MakeVector` 0.0 0.0 (`KismetMathLibrary.RandomFloatInRange` 0.0))) (0.0 0.0 0.0) (+ (`SceneComponent.K2_GetComponentLocation` (`|GetArrayItem` _instancemesh _returnvalue_3)) (`KismetMathLibrary.MakeVector` 0.0 0.0 (`KismetMathLibrary.RandomFloatInRange` 0.0))) (0.0 0.0 0.0) true)
          (`KismetArrayLibrary.Array_Add` (`self.InstanceSplineMesh`) _returnvalue_2))))))