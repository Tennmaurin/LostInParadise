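; BP_CaptureActor is a scene capture actor that follows the player and feeds capture data to the interactive grass material collection MPC_Grass.
; On BeginPlay it writes the capture's ortho width as CaptureSize and starts a fast looping timer.
; The timer moves it to player 0's XY at fixed height and writes CaptureLocation.
; It loops over GrassAffector-tagged components, but the show-only call is disconnected.
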(event `self.ReceiveBeginPlay`
  (`KismetMaterialLibrary.SetScalarParameterValue` "/Game/ART/Vegetation/InteractiveGrass_02/MPC_Grass.MPC_Grass" "CaptureSize" (`SceneCaptureComponent2D.OrthoWidth` (`self.SceneCaptureComponent2D`)))
  (`KismetSystemLibrary.K2_SetTimer` null "MoveTarget" 0.01 true)
  (bind _outactors (`GameplayStatics.GetAllActorsWithTag` "GrassAffector"))
  (for _array_element _outactors
    (for _array_element_2 (`self.GetComponentsByTag` _array_element "/Script/Engine.PrimitiveComponent" "GrassAffector")
      _)))

(event `MoveTarget`
  (bind (_returnvalue_x _returnvalue_y _returnvalue_z) (`KismetMathLibrary.BreakVector` (`self.K2_GetActorLocation`)))
  (bind (_returnvalue_x_2 _returnvalue_y_2) (`KismetMathLibrary.BreakVector` (`self.K2_GetActorLocation` (`GameplayStatics.GetPlayerCharacter` 0))))
  (`self.K2_SetActorLocation` (`KismetMathLibrary.MakeVector` _returnvalue_x_2 _returnvalue_y_2 _returnvalue_z))
  (`KismetMaterialLibrary.SetVectorParameterValue` "/Game/ART/Vegetation/InteractiveGrass_02/MPC_Grass.MPC_Grass" "CaptureLocation" (`KismetMathLibrary.Conv_VectorToLinearColor` (`self.K2_GetActorLocation`))))

(fn `UserConstructionScript`)